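; Shared function library for a calendar-driven sim game, providing game mode access, save handling and date math.
; The game mode is queried through GetGameModeMessage to expose player data, game data and TimeManager's current date and time.
; Save helpers load or create BP_PlayerData in a single default slot.
; Custom FDateTime helpers compare values, derive weekdays from a reference date, and offset by days, months or quarters using leap-year-aware month lengths.
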(fn `Add Days To Date`
  (params (Date :type "/Game/Blueprints/Structs/F_DateTime Structure") (`Days To Add` :type Integer))
  (returns (`New Date` :type "/Game/Blueprints/Structs/F_DateTime Structure"))
  (locals (`New Day` :type Integer) (`New Month ` :type Integer) (`New Year` :type Integer) (`Remaining Days` :type Integer))
  (bind (_day _month _year) (break `/Game/Blueprints/Structs/F_DateTime` Date))
  (bind (_day_2 _month_2 _year_2) (break `/Game/Blueprints/Structs/F_DateTime` Date))
  (bind (_day_3 _month_3 _year_3) (break `/Game/Blueprints/Structs/F_DateTime` Date))
  (bind _returnvalue (- (`self.Get Days In Month` _month _year) _day))
  (set `local.New Day` _day_3)
  (set `local.New Month ` _month_3)
  (set `local.New Year` _year_3)
  (bind _output_get (set `local.Remaining Days` `Days To Add`))
  (while (> _output_get 0)
    (if (<= (`local.Remaining Days`) _returnvalue)
      (return (make `/Game/Blueprints/Structs/F_DateTime` (+ (`local.Remaining Days`) _day_2) _month_2 _year_2))
      (else
        (bind _output_get_2 (set `local.Remaining Days` (- (`local.Remaining Days`) _returnvalue)))
        (set `local.New Day` _output_get_2)
        (set `local.Remaining Days` 0)
        (`/Engine/EditorBlueprintResources/StandardMacros.IncrementInt` (`local.New Month `)
          (:`  `
            (if (> (`local.New Month `) 12)
              (`/Engine/EditorBlueprintResources/StandardMacros.IncrementInt` (`local.New Year`)
                (:`  `
                  (set `local.New Month ` 1)))))))))
  (return (make `/Game/Blueprints/Structs/F_DateTime` (`local.New Day`) (`local.New Month `) (`local.New Year`))))

(fn `Add Months To Date`
  (params (`F Date Time` :type "/Game/Blueprints/Structs/F_DateTime Structure") (`Month To Add` :type Integer))
  (returns (`Date In Future Month` :type "/Game/Blueprints/Structs/F_DateTime Structure") (`Non Normalized Date In Future Month` :type "/Game/Blueprints/Structs/F_DateTime Structure"))
  (locals (`New Day` :type Integer) (`New Month` :type Integer) (`New Year` :type Integer) (`Remaining Months` :type Integer) (`Non Normalized Date` :type "/Game/Blueprints/Structs/F_DateTime Structure"))
  (bind (_day _month _year) (break `/Game/Blueprints/Structs/F_DateTime` `F Date Time`))
  (set `local.New Day` _day)
  (set `local.New Month` _month)
  (set `local.New Year` _year)
  (bind _output_get (set `local.Remaining Months` `Month To Add`))
  (while (> _output_get 0)
    (bind _result (`/Engine/EditorBlueprintResources/StandardMacros.IncrementInt` (`local.New Month`))
      (:`  `
        (if (> _result 12)
          (`/Engine/EditorBlueprintResources/StandardMacros.IncrementInt` (`local.New Year`)
            (:`  `
              (set `local.New Month` 1)
              (`/Engine/EditorBlueprintResources/StandardMacros.DecrementInt` (`local.Remaining Months`))))))))
  (`|ExecutionSequence`
    (:`then_0`
      (set `local.Non Normalized Date` (make `/Game/Blueprints/Structs/F_DateTime` (`local.New Day`) (`local.New Month`) (`local.New Year`))))
    (:`then_1`
      (set `local.New Day` (`KismetMathLibrary.Min` (`local.New Day`) (`self.Get Days In Month` (`local.New Month`) (`local.New Year`)))))
    (:`then_2`
      (return (make `/Game/Blueprints/Structs/F_DateTime` (`local.New Day`) (`local.New Month`) (`local.New Year`)) (`local.Non Normalized Date`)))))

(fn `Equal (Date & Time)`
  (params (A :type "/Game/Blueprints/Structs/F_DateTime Structure") (B :type "/Game/Blueprints/Structs/F_DateTime Structure"))
  (returns (`Return Value` :type Boolean))
  (bind (_day _month _year _hour _minute) (break `/Game/Blueprints/Structs/F_DateTime` A))
  (bind (_day_2 _month_2 _year_2 _hour_2 _minute_2) (break `/Game/Blueprints/Structs/F_DateTime` B))
  (return (and (== _day _day_2) (== _month _month_2) (== _year _year_2) (== _hour _hour_2) (== _minute _minute_2))))

(fn `Equal (Date)`
  (params (A :type "/Game/Blueprints/Structs/F_DateTime Structure") (B :type "/Game/Blueprints/Structs/F_DateTime Structure") (__WorldContext :type "Object Object Reference"))
  (returns (`Return Value` :type Boolean))
  (bind (_day _month _year) (break `/Game/Blueprints/Structs/F_DateTime` A))
  (bind (_day_2 _month_2 _year_2) (break `/Game/Blueprints/Structs/F_DateTime` B))
  (return (and (== _day _day_2) (== _month _month_2) (== _year _year_2))))

(fn `Equal (Time)`
  (params (A :type "/Game/Blueprints/Structs/F_DateTime Structure") (B :type "/Game/Blueprints/Structs/F_DateTime Structure") (__WorldContext :type "Object Object Reference"))
  (returns (`Return Value` :type Boolean))
  (bind (_day _month _year _hour _minute) (break `/Game/Blueprints/Structs/F_DateTime` A))
  (bind (_day_2 _month_2 _year_2 _hour_2 _minute_2) (break `/Game/Blueprints/Structs/F_DateTime` B))
  (return (and (== _hour _hour_2) (== _minute _minute_2))))

(fn `Get Current Date Time`
  (returns (`F Date Time` :type "/Game/Blueprints/Structs/F_DateTime Structure"))
  (bind _f_date_time (`/Game/Blueprints/Managers/BP_TimeManager.Get Date Time` (`/Game/Blueprints/BP_GameMode.Time Manager` (`self.Get Game Mode Sim` null))))
  (return _f_date_time))

(fn `Get Date In Next Quarter`
  (params (`F Date Time` :type "/Game/Blueprints/Structs/F_DateTime Structure"))
  (returns (`Date In Next Quarter` :type "/Game/Blueprints/Structs/F_DateTime Structure") (`Non Normalized Date In Future Quarter` :type "/Game/Blueprints/Structs/F_DateTime Structure"))
  (locals (`Months To Advance` :type Integer))
  (bind (_date_in_future_month _non_normalized_date_in_future_month) (`self.Add Months To Date` `F Date Time` (select `int` (`.Month_7_8DFEA87B4FB91E75FE6D15AEA2B32DAD` (break `/Game/Blueprints/Structs/F_DateTime` `F Date Time`)) :`0` 0 :`1` 3 :`2` 2 :`3` 1 :`4` 3 :`5` 2 :`6` 1 :`7` 3 :`8` 2 :`9` 1 :`10` 3 :`11` 2 :`12` 1)))
  (return _date_in_future_month _non_normalized_date_in_future_month))

(fn `Get Day Name From Date`
  (params (`F Date Time` :type "/Game/Blueprints/Structs/F_DateTime Structure"))
  (returns (Day :type "/Game/Blueprints/Enums/E_DayName Enum"))
  (locals (RefrenceDate :type "/Game/Blueprints/Structs/F_DateTime Structure" :default (struct :`Day` 1 :`Month` 1 :`Year` 2025)) (ReferenceDay :type "/Game/Blueprints/Enums/E_DayName Enum" :default "NewEnumerator2") (TotalDays :type Integer))
  (bind (_day _month _year) (break `/Game/Blueprints/Structs/F_DateTime` `F Date Time`))
  (`|ExecutionSequence`
    (:`then_0`
      (for _index (range (`.Year_8_DE12467241F4DDD386C28ABC72F09B02` (break `/Game/Blueprints/Structs/F_DateTime` (`local.RefrenceDate`))) _year)
        (set `local.TotalDays` (+ (`local.TotalDays`) (`KismetMathLibrary.SelectInt` 366 365 (`KismetMathLibrary.IsLeapYear` _index))))))
    (:`then_1`
      (for _index_2 (range 1 _month)
        (set `local.TotalDays` (+ (`local.TotalDays`) (`self.Get Days In Month` _index_2 _year)))))
    (:`then_2`
      (set `local.TotalDays` (+ (`local.TotalDays`) _day)))
    (:`then_3`
      (return (cast `/Game/Blueprints/Enums/E_DayName` (`KismetMathLibrary.Conv_IntToByte` (mod (- (+ (`local.TotalDays`) (`KismetMathLibrary.Conv_ByteToInt` (`local.ReferenceDay`))) 1) 7)))))))

(fn `Get Days In Month`
  (params (`Current Month` :type Integer) (`Current Year` :type Integer))
  (returns (`Days in current month` :type Integer))
  (switch `int` `Current Month`
    (:`1`
      _)
    (:`2`
      (return (`KismetMathLibrary.SelectInt` 29 28 (or (and (== (mod `Current Year` 4) 0) (!= (mod `Current Year` 100) 0)) (== (mod `Current Year` 400) 0)))))
    (:`3`
      _)
    (:`4`
      (return 30))
    (:`5`
      _)
    (:`6`
      (return 30))
    (:`7`
      _)
    (:`8`
      _)
    (:`9`
      (return 30))
    (:`10`
      _)
    (:`11`
      (return 30))
    (:`12`
      _))
  (return 31))

(fn `Get Game Mode Sim`
  (returns (`Game Mode Sim` :type "/Game/Blueprints/BP_GameMode Object Reference"))
  (bind _game_mode_sim (message `/Game/Blueprints/Interfaces/BPI_GameMode.GetGameMode` (`GameplayStatics.GetGameMode` null)))
  (return _game_mode_sim))

(fn `Get Next Date From Day Name`
  (params (`Day Name` :type "/Game/Blueprints/Enums/E_DayName Enum" :default "NewEnumerator0") (`F Date Time` :type "/Game/Blueprints/Structs/F_DateTime Structure"))
  (returns (`Next Date` :type "/Game/Blueprints/Structs/F_DateTime Structure"))
  (bind _returnvalue (- (`KismetMathLibrary.Conv_ByteToInt` `Day Name`) (`KismetMathLibrary.Conv_ByteToInt` (`self.Get Day Name From Date` `F Date Time`))))
  (return (`self.Add Days To Date` `F Date Time` (`KismetMathLibrary.SelectInt` (+ _returnvalue 7) _returnvalue (<= _returnvalue 0)))))

(fn `GetGameDataFromGM`
  (params (__WorldContext :type "Object Object Reference"))
  (returns (GameData :type "/Game/Blueprints/BP_GameData Object Reference"))
  (return (`/Game/Blueprints/BP_GameMode.GameData` (`self.Get Game Mode Sim` __WorldContext))))

(fn `GetNearestFloatInArray`
  (params (Array :type "Array of Float (double-precision)") (Value :type "Float (double-precision)"))
  (returns (`Nearest From Array` :type "Float (double-precision)"))
  (locals (ClosestValue :type "Float (double-precision)") (MinDiff :type "Float (double-precision)" :default 1e+19))
  (for _array_element Array
    (bind _returnvalue (`KismetMathLibrary.Abs` (- _array_element Value)))
    (if (< _returnvalue (`local.MinDiff`))
      (set `local.MinDiff` _returnvalue)
      (set `local.ClosestValue` _array_element)))
  (return (`local.ClosestValue`)))

(fn `GetPlayerDataFromGM`
  (returns (CurrentPlayerData :type "/Game/Blueprints/BP_PlayerData Object Reference"))
  (return (`/Game/Blueprints/BP_GameMode.CurrentPlayerData` (`self.Get Game Mode Sim` null))))

(fn `LoadGameFromSlot`
  (returns (`Player Data` :type "/Game/Blueprints/BP_PlayerData Object Reference"))
  (bind _returnvalue (`GameplayStatics.DoesSaveGameExist` "default"))
  (if _returnvalue
    (bind _returnvalue_2 (`GameplayStatics.LoadGameFromSlot` "default"))
    (bind _asbp_player_data (cast `/Game/Blueprints/BP_PlayerData` _returnvalue_2))
    (return _asbp_player_data)
    (else
      (bind _returnvalue_3 (`GameplayStatics.CreateSaveGameObject` "/Game/Blueprints/BP_PlayerData.BP_PlayerData_C"))
      (return _returnvalue_3))))

(fn `SaveGameToSlot`
  (params (PlayerData :type "/Game/Blueprints/BP_PlayerData Object Reference"))
  (returns (ReturnValue :type Boolean))
  (bind _returnvalue (`GameplayStatics.SaveGameToSlot` PlayerData "default"))
  (return _returnvalue))