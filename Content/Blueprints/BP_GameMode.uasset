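; BP_GameMode is the game mode that boots a session, loading saved player data and starting the main UI.
; On BeginPlay a sequence loads CurrentPlayerData from a save slot, then initializes TimeManager and FinanceManager with a reference to itself.
; It then creates WBP_GameUI, enables performance stats with a 60 FPS cap via console commands, and switches to UI-only input with a visible cursor.
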(event `self.ReceiveBeginPlay`
  (bind _returnvalue (`GameplayStatics.GetPlayerController` 0))
  (`|ExecutionSequence`
    (:`then_0`
      (bind _player_data (`/Game/Blueprints/BP_Lib.LoadGameFromSlot`))
      (set `self.CurrentPlayerData` _player_data))
    (:`then_1`
      (`self.Init`))
    (:`then_2`
      (bind _returnvalue_2 (`|CreateWidget` "/Game/Blueprints/UI/WBP_GameUI.WBP_GameUI_C"))
      (bind _output_get (set `self.GameUI` _returnvalue_2))
      (`UserWidget.AddToPlayerScreen` _output_get 1))
    (:`then_3`
      (`KismetSystemLibrary.ExecuteConsoleCommand` "stat unit" null)
      (`KismetSystemLibrary.ExecuteConsoleCommand` "stat fps" null)
      (`KismetSystemLibrary.ExecuteConsoleCommand` "t.MaxFPS 60" null))
    (:`then_4`
      (`WidgetBlueprintLibrary.SetInputMode_UIOnlyEx` _returnvalue (`self.GameUI`))
      (set `PlayerController.bShowMouseCursor` true _returnvalue))))

(event `Init`
  (`/Game/Blueprints/Managers/BP_TimeManager.Init` (`self.Time Manager`) self)
  (`/Game/Blueprints/Managers/BP_FinanceManager.Init` (`self.Finance Manager`) self))

(fn `GetGameMode`
  (returns (`Game Mode Sim` :type "/Game/Blueprints/BP_GameMode Object Reference"))
  (return self))

(fn `UserConstructionScript`)