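; BP_TimeManager runs the in-game calendar clock, advancing the minute, hour, day, month, quarter and year stored in the GameMode's current player data.
; Tick accumulates speed-scaled delta time unless paused, firing one game minute per configured tick delay in a catch-up loop.
; OnTick cascades rollovers, using real month lengths, and calls the matching tick notifications.
; A real-time check prints a recommended lower game speed when the loop overloads.
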(event `Init`
  (params (`Game Mode` :type "/Game/Blueprints/BP_GameMode Object Reference (by ref)"))
  (bind _output_get (set `self.GameMode` `Game Mode`))
  (bind _output_get_2 (set `self.Game Data` (`/Game/Blueprints/BP_GameMode.GameData` _output_get)))
  (set `self.DelayBetweenTicks` (`/Game/Blueprints/BP_GameData.DelayBetweenTicks` _output_get_2)))

(event `self.ReceiveTick`
  (params (DeltaSeconds :type "Float (single-precision)"))
  (bind (_seconds _partialseconds) (`GameplayStatics.GetAccurateRealTime`))
  (bind (_seconds_2 _partialseconds_2) (`GameplayStatics.GetAccurateRealTime`))
  (bind _currentplayerdata (`/Game/Blueprints/BP_GameMode.CurrentPlayerData` (`self.GameMode`)))
  (bind _currentplayerdata_2 (`/Game/Blueprints/BP_GameMode.CurrentPlayerData` (`self.GameMode`)))
  (bind _returnvalue (- (+ _seconds _partialseconds) (`self.CurrentUpdateTime`)))
  (if (and (not (`self.IsPaused`)) (> (`self.GameSpeedMultiplier`) 0.0))
    (bind _output_get (set `/Game/Blueprints/BP_PlayerData.TimeSinceLastMinute` (+ (`/Game/Blueprints/BP_PlayerData.TimeSinceLastMinute` _currentplayerdata_2) (* DeltaSeconds (`self.GameSpeedMultiplier`))) _currentplayerdata_2))
    (set `self.CurrentUpdateTime` (+ _seconds_2 _partialseconds_2))
    (while (> _output_get (`self.DelayBetweenTicks`))
      (set `/Game/Blueprints/BP_PlayerData.TimeSinceLastMinute` (- (`/Game/Blueprints/BP_PlayerData.TimeSinceLastMinute` _currentplayerdata) (`self.DelayBetweenTicks`)) _currentplayerdata)
      (`self.OnTick`)
      (set `self.RealFrameTime` _returnvalue)
      (if (> _returnvalue (* (`self.DelayBetweenTicks`) 0.9))
        (set `self.RecommendedGameSpeed` (/ (`self.DelayBetweenTicks`) (`self.RealFrameTime`)))
        ;[0.09809 0.15 0.000821 0.5] TODO: Tell player game is clamped
        (`KismetSystemLibrary.PrintString` (`KismetStringLibrary.Concat_StrStr` "The game is overloaded. Consider setting the game speed below x" (`KismetStringLibrary.Conv_DoubleToString` (`/Game/Blueprints/BP_Lib.GetNearestFloatInArray` (`/Game/Blueprints/BP_GameData.GameSpeedOptions` (`self.Game Data`)) (`self.RecommendedGameSpeed`)))))))))

(event `OnTick`
  (bind _currentplayerdata (`/Game/Blueprints/BP_GameMode.CurrentPlayerData` (`self.GameMode`)))
  (bind _currentmonth (`/Game/Blueprints/BP_PlayerData.CurrentMonth` _currentplayerdata))
  (`|ExecutionSequence`
    (:`then_0`
      (`/Engine/EditorBlueprintResources/StandardMacros.IncrementInt` (`/Game/Blueprints/BP_PlayerData.CurrentMinute` _currentplayerdata)))
    (:`then_1`
      (if (> (`/Game/Blueprints/BP_PlayerData.CurrentMinute` _currentplayerdata) 59)
        (set `/Game/Blueprints/BP_PlayerData.CurrentMinute` 0 _currentplayerdata)
        (bind _result (`/Engine/EditorBlueprintResources/StandardMacros.IncrementInt` (`/Game/Blueprints/BP_PlayerData.CurrentHour` _currentplayerdata))
          (:`  `
            (`self.OnHourTick` _result)))))
    (:`then_2`
      (if (> (`/Game/Blueprints/BP_PlayerData.CurrentHour` _currentplayerdata) 23)
        (set `/Game/Blueprints/BP_PlayerData.CurrentHour` 0 _currentplayerdata)
        (bind _result_2 (`/Engine/EditorBlueprintResources/StandardMacros.IncrementInt` (`/Game/Blueprints/BP_PlayerData.CurrentDay` _currentplayerdata))
          (:`  `
            (`self.OnDayTick` _result_2)))))
    (:`then_3`
      (if (> (`/Game/Blueprints/BP_PlayerData.CurrentDay` _currentplayerdata) (`/Game/Blueprints/BP_Lib.Get Days In Month` (`/Game/Blueprints/BP_PlayerData.CurrentMonth` _currentplayerdata) (`/Game/Blueprints/BP_PlayerData.CurrentYear` _currentplayerdata)))
        (`|ExecutionSequence`
          (:`then_0`
            (set `/Game/Blueprints/BP_PlayerData.CurrentDay` 1 _currentplayerdata)
            (bind _result_3 (`/Engine/EditorBlueprintResources/StandardMacros.IncrementInt` (`/Game/Blueprints/BP_PlayerData.CurrentMonth` _currentplayerdata))
              (:`  `
                (`self.OnMonthTick` _result_3))))
          (:`then_1`
            (if (or (== _currentmonth 1) (== _currentmonth 4) (== _currentmonth 7) (== _currentmonth 10))
              (bind _result_4 (`/Engine/EditorBlueprintResources/StandardMacros.IncrementInt` (`/Game/Blueprints/BP_PlayerData.CurrentQuarter` _currentplayerdata))
                (:`  `
                  (`self.OnQuarterTick` _result_4))))))))
    (:`then_4`
      (if (> (`/Game/Blueprints/BP_PlayerData.CurrentMonth` _currentplayerdata) 12)
        (set `/Game/Blueprints/BP_PlayerData.CurrentMonth` 1 _currentplayerdata)
        (bind _result_5 (`/Engine/EditorBlueprintResources/StandardMacros.IncrementInt` (`/Game/Blueprints/BP_PlayerData.CurrentYear` _currentplayerdata))
          (:`  `
            (`self.OnYearTick` _result_5)))))
    (:`then_5`
      (`self.OnMinuteTick` 0))))

(event `Set Game Speed Multiplier`
  (params (`New Speed Multiplier` :type "Float (double-precision)"))
  (if (>= `New Speed Multiplier` 0.0)
    (set `self.GameSpeedMultiplier` `New Speed Multiplier`)))

(fn `Get Date Time`
  (returns (`F Date Time` :type "/Game/Blueprints/Structs/F_DateTime Structure"))
  (bind _currentplayerdata (`/Game/Blueprints/BP_Lib.GetPlayerDataFromGM`))
  (return (make `/Game/Blueprints/Structs/F_DateTime` (`/Game/Blueprints/BP_PlayerData.CurrentDay` _currentplayerdata) (`/Game/Blueprints/BP_PlayerData.CurrentMonth` _currentplayerdata) (`/Game/Blueprints/BP_PlayerData.CurrentYear` _currentplayerdata) (`/Game/Blueprints/BP_PlayerData.CurrentHour` _currentplayerdata) (`/Game/Blueprints/BP_PlayerData.CurrentMinute` _currentplayerdata))))