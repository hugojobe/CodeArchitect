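; Finance manager that applies and records the player's immediate and recurring money transactions in player data.
; Transactions are stored in GUID-keyed maps; executing one adjusts CashBalance and adds a history entry.
; TimeManager's day tick runs daily items unconditionally and others on their next date, using non-normalized dates for month-based stepping.
; Rescheduled dates are set on the loop's struct without a map write-back, as a TODO notes.
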(event `Init`
  (params (`Game Mode` :type "/Game/Blueprints/BP_GameMode Object Reference (by ref)"))
  (bind _output_get (set `self.GameMode` `Game Mode`))
  (set `self.Game Data` (`/Game/Blueprints/BP_GameMode.GameData` _output_get))
  (add `/Game/Blueprints/Managers/BP_TimeManager.OnDayTick` (`/Game/Blueprints/BP_GameMode.Time Manager` _output_get) (delegate `On Day Tick`)))

(event `On Day Tick`
  (params (NewDay :type Integer))
  (`self.Check Recurrent Transactions` (`/Game/Blueprints/BP_Lib.Get Current Date Time`)))

(event `Check Recurrent Transactions`
  (params (`Current Date Time` :type "/Game/Blueprints/Structs/F_DateTime Structure"))
  (bind ((`RecurringSettings_39_42EE4237446B0B1AC4471CACD5049B85` _recurringsettings)) (break `/Game/Blueprints/Structs/F_TransactionData` (struct)))
  (bind (_next_execution_date _non_normalized_next_execution_date) (`self.Calculate Next Recurring Execution Date` _recurringsettings))
  (bind (_day _month _year) (break `/Game/Blueprints/Structs/F_DateTime` (`.NextExecutionDate_26_70C717FC498BB2E2489032ABD6728BB3` (break `/Game/Blueprints/Structs/F_RecurringSettings` _recurringsettings))))
  (bind (_keypin _valuepin) (`|MapForEach` (`/Game/Blueprints/BP_PlayerData.ActiveRecurrentTransactions` (`/Game/Blueprints/BP_Lib.GetPlayerDataFromGM`)))
    (:`then`
      (bind (_transactiontype _amount _description _executeimmediately _transactionid _category _daterecorded _isrecurrent _recurringsettings_2) (break `/Game/Blueprints/Structs/F_TransactionData` _valuepin))
      (bind (_frequency _startexecutiondate _nextexecutiondate) (break `/Game/Blueprints/Structs/F_RecurringSettings` _recurringsettings_2))
      (if (`|EnumEquality` _frequency "NewEnumerator0")
        (`self.Execute Immediate Transaction` _transactiontype _category _amount _description :!label _label)
        (elif (`/Game/Blueprints/BP_Lib.Equal (Date)` `Current Date Time` _nextexecutiondate)
          (`|ExecutionSequence`
            (:`then_0`
              (goto _label))
            (:`then_1`
              (bind _structout (setmembers `/Game/Blueprints/Structs/F_RecurringSettings` :`StructRef` _recurringsettings :`Next Execution Date` _next_execution_date :`Non Normalized Next Execution Date` _non_normalized_next_execution_date))
              (bind (_day_2 _month_2 _year_2) (break `/Game/Blueprints/Structs/F_DateTime` (`.NextExecutionDate_26_70C717FC498BB2E2489032ABD6728BB3` (break `/Game/Blueprints/Structs/F_RecurringSettings` _structout))))
              (`KismetSystemLibrary.PrintString` (`KismetStringLibrary.Concat_StrStr` "Executed recurrent transaction, next date is: " (`KismetStringLibrary.Conv_IntToString` _day_2) "/" (`KismetStringLibrary.Conv_IntToString` _month_2) "/" (`KismetStringLibrary.Conv_IntToString` _year_2)) true true (struct :`R` 1.0 :`G` 0.59251 :`A` 1.0) 200000.0)
              (`KismetSystemLibrary.PrintString` (`KismetStringLibrary.Concat_StrStr` "next date is: " (`KismetStringLibrary.Conv_IntToString` _day) "/" (`KismetStringLibrary.Conv_IntToString` _month) "/" (`KismetStringLibrary.Conv_IntToString` _year)) true true (struct :`R` 1.0 :`G` 0.058848 :`A` 1.0) 200000.0))))))))

(fn `Add Reccurent Transaction`
  (params (`Transaction Type` :type "/Game/Blueprints/Enums/E_TransactionType Enum" :default "NewEnumerator0") (Frequency :type "/Game/Blueprints/Enums/E_TimeFrequence Enum" :default "NewEnumerator0") (Category :type "/Game/Blueprints/Enums/E_FinanceCategory Enum" :default "NewEnumerator1") (Amount :type "Float (double-precision)") (Description :type Text) (`Start Execution Date` :type "/Game/Blueprints/Structs/F_DateTime Structure") (`Also Execute Today` :type Boolean))
  (returns (Success :type Boolean) (`Transaction Guid` :type "Guid Structure"))
  (`|ExecutionSequence`
    (:`then_0`
      (bind _output_get (set `self.Guid` (`KismetGuidLibrary.NewGuid`)))
      (`KismetSystemLibrary.PrintString` (`KismetGuidLibrary.Conv_GuidToString` _output_get))
      (`BlueprintMapLibrary.Map_Add` (`/Game/Blueprints/BP_PlayerData.ActiveRecurrentTransactions` (`/Game/Blueprints/BP_Lib.GetPlayerDataFromGM`)) (`self.Guid`) (make `/Game/Blueprints/Structs/F_TransactionData` `Transaction Type` Amount Description `Also Execute Today` (`self.Guid`) Category (`/Game/Blueprints/BP_Lib.Get Current Date Time`) true (make `/Game/Blueprints/Structs/F_RecurringSettings` Frequency `Start Execution Date` `Start Execution Date` `Start Execution Date`))))
    (:`then_1`
      (if `Also Execute Today`
        (`self.Execute Immediate Transaction` `Transaction Type` Category Amount Description)))
    (:`then_2`
      (return true (`self.Guid`)))))

(fn `Calculate Next Recurring Execution Date`
  (params (`Recurring Settings` :type "/Game/Blueprints/Structs/F_RecurringSettings Structure"))
  (returns (`Next Execution Date` :type "/Game/Blueprints/Structs/F_DateTime Structure") (`Non Normalized Next Execution Date` :type "/Game/Blueprints/Structs/F_DateTime Structure"))
  (locals (MonthToAdd :type Integer) (NextDate :type "/Game/Blueprints/Structs/F_DateTime Structure"))
  (bind (_frequency _startexecutiondate _nextexecutiondate _nonnormalizednextexecutiondate) (break `/Game/Blueprints/Structs/F_RecurringSettings` `Recurring Settings`))
  (bind (_date_in_future_month _non_normalized_date_in_future_month) (`/Game/Blueprints/BP_Lib.Add Months To Date` _nonnormalizednextexecutiondate 1))
  (bind _new_date (`/Game/Blueprints/BP_Lib.Add Days To Date` _nextexecutiondate 1))
  (bind (_date_in_future_month_2 _non_normalized_date_in_future_month_2) (`/Game/Blueprints/BP_Lib.Add Months To Date` _nonnormalizednextexecutiondate 12))
  (bind (_date_in_next_quarter _non_normalized_date_in_future_quarter) (`/Game/Blueprints/BP_Lib.Get Date In Next Quarter` _nonnormalizednextexecutiondate))
  (bind _next_date (`/Game/Blueprints/BP_Lib.Get Next Date From Day Name` (`/Game/Blueprints/BP_Lib.Get Day Name From Date` _startexecutiondate) _nextexecutiondate))
  (switch `/Game/Blueprints/Enums/E_TimeFrequence` _frequency
    (:`NewEnumerator0`
      (return _new_date _new_date))
    (:`NewEnumerator1`
      (return _next_date _next_date))
    (:`NewEnumerator2`
      (return _date_in_future_month _non_normalized_date_in_future_month))
    (:`NewEnumerator3`
      (return _date_in_next_quarter _non_normalized_date_in_future_quarter))
    (:`NewEnumerator4`
      (return _date_in_future_month_2 _non_normalized_date_in_future_month_2))))

(fn `Execute Immediate Transaction`
  (params (`Transaction Type` :type "/Game/Blueprints/Enums/E_TransactionType Enum" :default "NewEnumerator0") (Category :type "/Game/Blueprints/Enums/E_FinanceCategory Enum" :default "NewEnumerator1") (Amount :type "Float (double-precision)") (Description :type Text))
  (returns (Success :type Boolean) (`Transaction Guid` :type "Guid Structure"))
  (bind _currentplayerdata (`/Game/Blueprints/BP_Lib.GetPlayerDataFromGM`))
  (`|ExecutionSequence`
    (:`then_0`
      (set `self.Guid` (`KismetGuidLibrary.NewGuid`))
      (set `/Game/Blueprints/BP_PlayerData.CashBalance` (+ (`/Game/Blueprints/BP_PlayerData.CashBalance` _currentplayerdata) (* (`KismetMathLibrary.Abs` Amount) (`KismetMathLibrary.SelectFloat` 1.0 -1.0 (`|EnumEquality` `Transaction Type` "NewEnumerator1")))) _currentplayerdata))
    (:`then_1`
      (`BlueprintMapLibrary.Map_Add` (`/Game/Blueprints/BP_PlayerData.TransactionHistory` (`/Game/Blueprints/BP_Lib.GetPlayerDataFromGM`)) (`self.Guid`) (make `/Game/Blueprints/Structs/F_TransactionData` `Transaction Type` (`KismetMathLibrary.Abs` Amount) Description true (`self.Guid`) Category (`/Game/Blueprints/BP_Lib.Get Current Date Time`) false (struct :`Frequency` "NewEnumerator0" :`StartExecutionDate` (struct) :`NextExecutionDate` (struct) :`NonNormalizedNextExecutionDate` (struct)))))
    (:`then_2`
      (`KismetSystemLibrary.PrintString` (`KismetTextLibrary.Conv_TextToString` Description))
      (return true (`self.Guid`)))))

(fn `Get Active Recurrent Transaction From Guid`
  (params (Guid :type "Guid Structure"))
  (returns (Success :type Boolean) (`Transaction Data` :type "/Game/Blueprints/Structs/F_TransactionData Structure"))
  (bind (_value _returnvalue) (`BlueprintMapLibrary.Map_Find` (`/Game/Blueprints/BP_PlayerData.ActiveRecurrentTransactions` (`/Game/Blueprints/BP_Lib.GetPlayerDataFromGM`)) Guid))
  (return _returnvalue _value))

(fn `Get Transaction From History`
  (params (Guid :type "Guid Structure"))
  (returns (Success :type Boolean) (`Transaction Data` :type "/Game/Blueprints/Structs/F_TransactionData Structure"))
  (bind (_value _returnvalue) (`BlueprintMapLibrary.Map_Find` (`/Game/Blueprints/BP_PlayerData.TransactionHistory` (`/Game/Blueprints/BP_Lib.GetPlayerDataFromGM`)) Guid))
  (return _returnvalue _value))